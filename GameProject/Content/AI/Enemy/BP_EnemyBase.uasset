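; Base enemy character that supplies attack, weapon handling, patrol route, ideal combat ranges and movement speed functions.
; Attack plays a montage and fires OnAttackEnd whether it completes or is interrupted.
; Montage notifies time the weapon swap, spawning a BP_Arrow onto the left-hand socket or destroying it, with OnSheatheWeapon fired when sheathing completes.
; SetMovementSpeed maps named movement states to walk speeds.
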(event `Attack`
  (`|PlayMontage` (`self.Mesh`) "/Game/AI/Enemy/Animations/AttackMontage.AttackMontage" 2.0
    (:`OnCompleted`
      _)
    (:`OnInterrupted`
      _))
  (`self.OnAttackEnd`))

(event `WieldWeapon`
  (bind _notifyname (`|PlayMontage` (`self.Mesh`) "/Game/AI/Enemy/Animations/UnsheathingMontage.UnsheathingMontage")
    (:`OnNotifyBegin`
      (switch `name` _notifyname
        (:`UnsheatheWeapon`
          (bind _returnvalue (`|SpawnActorFromClass` "/Game/AI/Weapons/BP_Arrow.BP_Arrow_C" (`self.GetTransform`) "Undefined" "MultiplyWithRoot" null null))
          (bind _output_get (set `self.WeaponActor` _returnvalue))
          (`self.K2_AttachToComponent` _output_get (`self.Mesh`) "LeftHandWeaponSocket" "SnapToTarget" "SnapToTarget" "SnapToTarget" true)
          (set `self.IsWieldingWeapon` true))))))

(event `SheatheWeapon`
  (bind _notifyname (`|PlayMontage` (`self.Mesh`) "/Game/AI/Enemy/Animations/SheathingWeaponMontage.SheathingWeaponMontage" 1.0 0.3)
    (:`OnCompleted`
      (`self.OnSheatheWeapon`))
    (:`OnNotifyBegin`
      (switch `name` _notifyname
        (:`SheatheWeapon`
          (`self.K2_DestroyActor` (`self.WeaponActor`))
          (set `self.IsWieldingWeapon` false))))))

(fn `GetIdealRange`
  (returns (AttackRadius :type "Float (double-precision)") (DefendRadius :type "Float (double-precision)"))
  (return 100.0 350.0))

(fn `GetPatrolRoute`
  (returns (PatrolRoute :type "/Game/AI/Enemy/BT_Enemies/BP_PatrolRoute Object Reference"))
  (return (`self.PatrolRoute`)))

(fn `SetMovementSpeed`
  (params (Speed :type "/Game/AI/Enums/E_MovementSpeed Enum (by ref)" :default "NewEnumerator0"))
  (returns (SpeedValue :type "Float (double-precision)"))
  (set `CharacterMovementComponent.MaxWalkSpeed` (select `/Game/AI/Enums/E_MovementSpeed` Speed :`NewEnumerator0` 50.0 :`NewEnumerator1` 100.0 :`NewEnumerator2` 300.0 :`NewEnumerator3` 500.0 :!type "Float (single-precision)") (`self.CharacterMovement`))
  (return 0.0))

(fn `UserConstructionScript`)
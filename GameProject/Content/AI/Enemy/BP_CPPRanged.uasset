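; Ranged enemy AI Blueprint that supplies the attack behavior, apparently on top of C++ logic.
; Attack plays the attack montage on the mesh at increased rate and calls OnAttackEnd whether it completes or is interrupted.
; SetMovementSpeed is a stub that ignores its input and returns zero, and the weapon wield and sheathe calls are never executed.
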(event `self.Attack`
  (`|PlayMontage` (`self.Mesh`) "/Game/AI/Enemy/Animations/AttackMontage.AttackMontage" 2.0
    (:`OnCompleted`
      _)
    (:`OnInterrupted`
      _))
  (`self.OnAttackEnd`))

(fn `SetMovementSpeed`
  (params (Speed :type "/Game/AI/Enums/E_MovementSpeed Enum (by ref)" :default "NewEnumerator0"))
  (returns (SpeedValue :type "Float (double-precision)"))
  (return 0.0))

(fn `UserConstructionScript`
  (`parent.UserConstructionScript`))